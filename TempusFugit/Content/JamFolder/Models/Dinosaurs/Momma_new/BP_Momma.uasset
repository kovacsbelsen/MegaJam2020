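; BP_Momma is the mother dinosaur character that catches and eats the player.
; It caches the MainChar on BeginPlay; EatPlayer stops its own movement, dismounts the player if riding a dino, then possesses Momma with the player controller.
; The player loses mesh collision and movement, snaps to Momma's PlayerSocket and is marked dead, followed by a brief global slow-motion before time returns to normal.
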(event `self.ReceiveBeginPlay`
  (bind _returnvalue (`GameplayStatics.GetActorOfClass` "/Game/JamFolder/Blueprints/MainChar.MainChar_C"))
  (set `self.PlayerReference` _returnvalue))

(event `Eat Player`
  (bind _playerreference (`self.PlayerReference`))
  (bind _playerreference_2 (`self.PlayerReference`))
  (bind _charactermovement (`Character.CharacterMovement` _playerreference))
  (`CharacterMovementComponent.DisableMovement` (`self.CharacterMovement`))
  (if (`/Game/JamFolder/Blueprints/MainChar.IsRidingDino` (`self.PlayerReference`))
    (`self.K2_DetachFromActor` _playerreference_2 "KeepWorld" "KeepWorld" "KeepWorld")
    (set `/Game/JamFolder/Blueprints/MainChar.IsRidingDino` false _playerreference_2))
  (`Controller.Possess` (`GameplayStatics.GetPlayerController` 0) self)
  (`PrimitiveComponent.SetCollisionEnabled` (`Character.Mesh` _playerreference) "NoCollision")
  (`NavMovementComponent.StopActiveMovement` _charactermovement)
  (`CharacterMovementComponent.DisableMovement` _charactermovement)
  (`self.K2_AttachToComponent` _playerreference (`self.Mesh`) "PlayerSocket" "SnapToTarget" "SnapToTarget" "KeepWorld" true)
  (set `/Game/JamFolder/Blueprints/MainChar.IsDead` true _playerreference)
  (`GameplayStatics.SetGlobalTimeDilation` 0.2)
  (`KismetSystemLibrary.Delay` 0.7)
  (`GameplayStatics.SetGlobalTimeDilation` 1.0))

(fn `UserConstructionScript`)