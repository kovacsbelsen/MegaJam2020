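; BP_FallingTree is a tree actor that topples away from BP_Momma the first time she overlaps its trigger sphere.
; On that overlap it stores the direction from her capsule to the sphere and starts a looping timer at about 30 Hz.
; Each tick increases the angle by FallingSpeed, rotating the actor around the cross product of world up and that direction, until it reaches 85 degrees and clears the timer.
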(event `self.Sphere.OnComponentBeginOverlap`
  (params (OverlappedComponent :type "PrimitiveComponent Object Reference") (OtherActor :type "Actor Object Reference") (OtherComp :type "PrimitiveComponent Object Reference") (OtherBodyIndex :type Integer) (bFromSweep :type Boolean) (SweepResult :type "HitResult Structure (by ref)"))
  (bind _asbp_momma (cast `/Game/JamFolder/Models/Dinosaurs/Momma_new/BP_Momma` OtherActor))
  (`/Engine/EditorBlueprintResources/StandardMacros.DoOnce` false
    (:`Completed`
      (`|ExecutionSequence`
        (:`then_0`
          (set `self.direction` (`KismetMathLibrary.Normal` (- (`SceneComponent.K2_GetComponentLocation` (`self.Sphere`)) (`SceneComponent.K2_GetComponentLocation` (`Character.CapsuleComponent` _asbp_momma))))))
        (:`then_1`
          (bind _returnvalue (`KismetSystemLibrary.K2_SetTimerDelegate` (delegate `FallingTree`) 0.033333 true))
          (bind _output_get (set `self.FallingTimer` _returnvalue)))))))

(event `FallingTree`
  (bind _output_get (set `self.rotation` (+ (`self.rotation`) (`self.FallingSpeed`))))
  (`self.K2_SetActorRotation` (`KismetMathLibrary.RotatorFromAxisAndAngle` (`KismetMathLibrary.Cross_VectorVector` (0.0 0.0 1.0) (`self.direction`)) _output_get))
  (if (>= (`self.rotation`) 85.0)
    (`KismetSystemLibrary.K2_ClearAndInvalidateTimerHandle` (stale `self.Sphere.OnComponentBeginOverlap` _output_get))))

(fn `UserConstructionScript`)