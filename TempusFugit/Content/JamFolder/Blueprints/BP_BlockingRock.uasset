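; BP_BlockingRock is a rock obstacle that the player pushes aside by pressing Space Bar when prompted.
; The first MainChar overlap with its trigger disables character movement, shows an animated PushRock_Widget and enables input on the rock.
; Space Bar reverses the widget animation, removes it after a delay and disables the rock's input.
; The RockMovement timeline then yaws RockPivot and restores walking when finished.
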(event `self.PlayerTrigger.OnComponentBeginOverlap`
  (params (OverlappedComponent :type "PrimitiveComponent Object Reference") (OtherActor :type "Actor Object Reference") (OtherComp :type "PrimitiveComponent Object Reference") (OtherBodyIndex :type Integer) (bFromSweep :type Boolean) (SweepResult :type "HitResult Structure (by ref)"))
  (bind _asmain_char (cast `/Game/JamFolder/Blueprints/MainChar` OtherActor))
  (`/Engine/EditorBlueprintResources/StandardMacros.DoOnce` false
    (:`Completed`
      (`CharacterMovementComponent.DisableMovement` (`Character.CharacterMovement` _asmain_char))
      (bind _returnvalue (`|CreateWidget` "/Game/JamFolder/UI/PushRock_Widget.PushRock_Widget_C"))
      (bind _output_get (set `self.WidgetReference` _returnvalue))
      (`UserWidget.AddToViewport` _output_get 0)
      (`UserWidget.PlayAnimation` _returnvalue (`/Game/JamFolder/UI/PushRock_Widget.BlendIn` _returnvalue) 0.0 1 "Forward" 1.0 false)
      (`self.EnableInput` (`GameplayStatics.GetPlayerController` 0)))))

(event `Key|SpaceBar`
  (params (Key :type "Key Structure"))
  (bind _widgetreference (`self.WidgetReference`))
  (:`Pressed`
    (`UserWidget.PlayAnimation` _widgetreference null 0.0 1 "Reverse" 1.0 false)
    (`KismetSystemLibrary.Delay` (`WidgetAnimation.GetEndTime` (`/Game/JamFolder/UI/PushRock_Widget.BlendIn` _widgetreference)))
    (`Widget.RemoveFromParent` (`self.WidgetReference`))
    (`self.DisableInput` (`GameplayStatics.GetPlayerController` 0))
    (`self.MoveRock`)))

(event `MoveRock`
  (bind (_direction _zrot) (`Timeline|RockMovement`)
    (:`Update`
      (`SceneComponent.K2_SetRelativeRotation` (`self.RockPivot`) (`KismetMathLibrary.MakeRotator` 0.0 0.0 _zrot) false false))
    (:`Finished`
      (bind _asmain_char (cast `/Game/JamFolder/Blueprints/MainChar` (`GameplayStatics.GetPlayerCharacter` 0)))
      (`CharacterMovementComponent.SetMovementMode` (`Character.CharacterMovement` _asmain_char) "MOVE_Walking" 0))))

(fn `UserConstructionScript`)