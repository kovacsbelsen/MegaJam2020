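; BP_FallingRock is a one-shot rock trap that topples when MainChar overlaps its trigger and can crush the player.
; A short looping timer repeatedly pushes the Cube along world -Y, scaled by PushForce, leaving the fall to physics.
; Hits on MainChar or BP_Baby share a speed and height-above-character check before KillPlayer.
; KillPlayer detaches a dino rider, disables the character, triggers death, unpossesses the controller and plays brief slow motion.
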(event `Test`
  ;[0.3158 1 0.1369] Falling Trigger
  (bind _returnvalue (`KismetSystemLibrary.K2_SetTimerDelegate` (delegate `PushRock`) 0.033333 true :!label _label))
  (`KismetSystemLibrary.Delay` 0.5)
  (`KismetSystemLibrary.K2_ClearAndInvalidateTimerHandle` _returnvalue))

(event `self.TrapTrigger.OnComponentBeginOverlap`
  (params (OverlappedComponent :type "PrimitiveComponent Object Reference") (OtherActor :type "Actor Object Reference") (OtherComp :type "PrimitiveComponent Object Reference") (OtherBodyIndex :type Integer) (bFromSweep :type Boolean) (SweepResult :type "HitResult Structure (by ref)"))
  ;[0.3158 1 0.1369] Falling Trigger
  (cast `/Game/JamFolder/Blueprints/MainChar` OtherActor)
  (`/Engine/EditorBlueprintResources/StandardMacros.DoOnce` false
    (:`Completed`
      (goto _label))))

(event `PushRock`
  ;[0.3158 1 0.1369] Falling Trigger
  (`PrimitiveComponent.AddForce` (`self.Cube`) (* (`KismetMathLibrary.MakeVector` 0.0 -1.0) (* 500000.0 (`self.PushForce`))) "None" false))

(event `self.Cube.OnComponentHit`
  (params (HitComponent :type "PrimitiveComponent Object Reference") (OtherActor :type "Actor Object Reference") (OtherComp :type "PrimitiveComponent Object Reference") (NormalImpulse :type "Vector Structure") (Hit :type "HitResult Structure (by ref)"))
  (bind (_returnvalue_x _returnvalue_y _returnvalue_z) (`KismetMathLibrary.BreakVector` (`SceneComponent.K2_GetComponentLocation` (`self.Cube`))))
  ;[0.2673 0.4129 1] Hit Check
  (bind _asmain_char (cast `/Game/JamFolder/Blueprints/MainChar` OtherActor)
    (:`then`
      _)
    (:`CastFailed`
      (cast `/Game/JamFolder/Models/Dinosaurs/Baby_new/BP_Baby` OtherActor)))
  (bind (_returnvalue_x_2 _returnvalue_y_2 _returnvalue_z_2) (`KismetMathLibrary.BreakVector` (`SceneComponent.K2_GetComponentLocation` (`Character.CapsuleComponent` _asmain_char))))
  (if (and (> (`KismetMathLibrary.VSize` (`SceneComponent.GetComponentVelocity` (`self.Cube`))) 400.0) (> _returnvalue_z (+ _returnvalue_z_2 100.0)))
    (`/Engine/EditorBlueprintResources/StandardMacros.DoOnce` false
      (:`Completed`
        (`self.KillPlayer`)))))

(event `KillPlayer`
  ;[1 0.1011 0.05795] Kill the Player
  (bind _returnvalue (`GameplayStatics.GetActorOfClass` "/Game/JamFolder/Blueprints/MainChar.MainChar_C"))
  (if (`/Game/JamFolder/Blueprints/MainChar.IsRidingDino` _returnvalue)
    (`self.K2_DetachFromActor` _returnvalue "KeepWorld" "KeepWorld" "KeepWorld")
    (set `/Game/JamFolder/Blueprints/MainChar.IsRidingDino` false _returnvalue)
    (`self.K2_AddActorWorldOffset` _returnvalue (0.0 0.0 -20.0) false true))
  (`PrimitiveComponent.SetCollisionEnabled` (`Character.Mesh` _returnvalue) "NoCollision")
  (bind _charactermovement (`Character.CharacterMovement` _returnvalue))
  (`NavMovementComponent.StopActiveMovement` _charactermovement)
  (`CharacterMovementComponent.DisableMovement` _charactermovement)
  (set `/Game/JamFolder/Blueprints/MainChar.IsDead` true _returnvalue)
  (`/Game/JamFolder/Blueprints/MainChar.PlayerDie` _returnvalue)
  (`Controller.UnPossess` (`GameplayStatics.GetPlayerController` 0))
  (`GameplayStatics.SetGlobalTimeDilation` 0.2)
  (`KismetSystemLibrary.Delay` 0.7)
  (`GameplayStatics.SetGlobalTimeDilation` 1.0))

(fn `UserConstructionScript`)