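; BP_Lava is a lava hazard that kills the player when either MainChar or a BP_Baby touches its KillCollision.
; A baby overlap kills the player that baby references, and a DoOnce limits the death to one trigger.
; KillPlayer detaches a dino-riding player, disables mesh collision and movement, calls PlayerDie and unpossesses the controller.
; A brief global slow-motion plays before time dilation returns to normal.
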(event `self.KillCollision.OnComponentBeginOverlap`
  (params (OverlappedComponent :type "PrimitiveComponent Object Reference") (OtherActor :type "Actor Object Reference") (OtherComp :type "PrimitiveComponent Object Reference") (OtherBodyIndex :type Integer) (bFromSweep :type Boolean) (SweepResult :type "HitResult Structure (by ref)"))
  (bind _asmain_char (cast `/Game/JamFolder/Blueprints/MainChar` OtherActor)
    (:`then`
      (set `self.PlayerReference` _asmain_char))
    (:`CastFailed`
      (bind _asbp_baby (cast `/Game/JamFolder/Models/Dinosaurs/Baby_new/BP_Baby` OtherActor))
      (set `self.PlayerReference` (`/Game/JamFolder/Models/Dinosaurs/Baby_new/BP_Baby.PlayerReference` _asbp_baby))))
  (`/Engine/EditorBlueprintResources/StandardMacros.DoOnce` false
    (:`Completed`
      (`self.KillPlayer`))))

(event `KillPlayer`
  (bind _playerreference (`self.PlayerReference`))
  (bind _charactermovement (`Character.CharacterMovement` _playerreference))
  (if (`/Game/JamFolder/Blueprints/MainChar.IsRidingDino` _playerreference)
    (`self.K2_DetachFromActor` _playerreference "KeepWorld" "KeepWorld" "KeepWorld")
    (set `/Game/JamFolder/Blueprints/MainChar.IsRidingDino` false _playerreference)
    (`self.K2_AddActorWorldOffset` _playerreference (0.0 0.0 -20.0) false true))
  (`PrimitiveComponent.SetCollisionEnabled` (`Character.Mesh` _playerreference) "NoCollision")
  (`NavMovementComponent.StopActiveMovement` _charactermovement)
  (`CharacterMovementComponent.DisableMovement` _charactermovement)
  (set `/Game/JamFolder/Blueprints/MainChar.IsDead` true _playerreference)
  (`/Game/JamFolder/Blueprints/MainChar.PlayerDie` _playerreference)
  (`Controller.UnPossess` (`GameplayStatics.GetPlayerController` 0))
  (`GameplayStatics.SetGlobalTimeDilation` 0.2)
  (`KismetSystemLibrary.Delay` 0.7)
  (`GameplayStatics.SetGlobalTimeDilation` 1.0))

(fn `UserConstructionScript`)