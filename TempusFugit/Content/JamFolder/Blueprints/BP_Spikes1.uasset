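; Spike hazard that hurts the MainChar when it overlaps the Box.
; A hit drops a hanging player from the ledge, disables input, launches them back and up, spawns an impact effect and removes a heart.
; It also sets the character's condition, switching it again when health is depleted.
; A DoOnce reset after a short delay limits repeat hits; the EnableInput call here is disconnected.
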(event `CanBeDamagedAgain`
  (bind _playerref (`self.PlayerRef`))
  (bind _playerref_2 (`self.PlayerRef`))
  (bind (_returnvalue_x _returnvalue_y) (`KismetMathLibrary.BreakVector` (`self.GetActorForwardVector` (`self.PlayerRef`))))
  (goto _label :!via `Reset`))

(event `self.Box.OnComponentBeginOverlap`
  (params (OverlappedComponent :type "PrimitiveComponent Object Reference") (OtherActor :type "Actor Object Reference") (OtherComp :type "PrimitiveComponent Object Reference") (OtherBodyIndex :type Integer) (bFromSweep :type Boolean) (SweepResult :type "HitResult Structure (by ref)"))
  (bind _playerref (`self.PlayerRef`))
  (bind _playerref_2 (`self.PlayerRef`))
  (bind (_returnvalue_x _returnvalue_y) (`KismetMathLibrary.BreakVector` (`self.GetActorForwardVector` (`self.PlayerRef`))))
  (bind _asmain_char (cast `/Game/JamFolder/Blueprints/MainChar` OtherActor))
  (bind _output_get (set `self.PlayerRef` _asmain_char))
  (`/Engine/EditorBlueprintResources/StandardMacros.DoOnce` false :!label _label
    (:`Completed`
      (if (`/Game/JamFolder/Blueprints/MainChar.IsHanging?` (`self.PlayerRef`))
        (`/Game/JamFolder/Blueprints/MainChar.GetOffLedge` (`self.PlayerRef`)))
      (`self.DisableInput` _output_get (`GameplayStatics.GetPlayerController` 0))
      (`Character.LaunchCharacter` _playerref_2 (`KismetMathLibrary.MakeVector` (* _returnvalue_x -500.0) (* _returnvalue_y -500.0) 300.0) true true)
      (set `/Game/JamFolder/Blueprints/MainChar.CharacterCondition` "NewEnumerator0" (`self.PlayerRef`))
      (`GameplayStatics.SpawnEmitterAtLocation` "/Game/PlatformerDevelopmentKit/Characters/Player/Particles/PS_Impact.PS_Impact" (`self.K2_GetActorLocation` _playerref_2))
      (`/Game/JamFolder/UI/Main_Widget.UpdateHearts` (`/Game/JamFolder/Blueprints/MainChar.MainWidgetReference` (`self.PlayerRef`)) -1)
      (if (<= (`/Game/JamFolder/Blueprints/MainChar.CurrentHealth` (`self.PlayerRef`)) 0)
        (set `/Game/JamFolder/Blueprints/MainChar.CharacterCondition` "NewEnumerator1" _playerref)
        (`self.DisableInput` _playerref (`GameplayStatics.GetPlayerController` 0))
        (`KismetSystemLibrary.Delay` 0.5)
        (`self.CanBeDamagedAgain`)
        (else
          (`KismetSystemLibrary.Delay` 0.5)
          (`self.CanBeDamagedAgain`))))))

(fn `UserConstructionScript`)