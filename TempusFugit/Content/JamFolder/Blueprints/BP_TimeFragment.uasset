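; BP_TimeFragment is a collectible pickup that the player character gathers by touching its sphere.
; On overlap with MainChar it disables the sphere's collision, increments the character's CoinAmount and refreshes the coin display on the main widget.
; It then spawns the CollectTimeFrame emitter at the sphere's location and destroys itself immediately.
; A disconnected chain for a pickup animation and delayed emitter cleanup never runs.
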(event `self.Sphere.OnComponentBeginOverlap`
  (params (OverlappedComponent :type "PrimitiveComponent Object Reference") (OtherActor :type "Actor Object Reference") (OtherComp :type "PrimitiveComponent Object Reference") (OtherBodyIndex :type Integer) (bFromSweep :type Boolean) (SweepResult :type "HitResult Structure (by ref)"))
  (bind _asmain_char (cast `/Game/JamFolder/Blueprints/MainChar` OtherActor))
  (`PrimitiveComponent.SetCollisionResponseToAllChannels` (`self.Sphere`) "ECR_Ignore")
  (set `/Game/JamFolder/Blueprints/MainChar.CoinAmount` (+ (`/Game/JamFolder/Blueprints/MainChar.CoinAmount` _asmain_char) 1) _asmain_char)
  (`/Game/JamFolder/UI/Main_Widget.UpdateCoins` (`/Game/JamFolder/Blueprints/MainChar.MainWidgetReference` _asmain_char))
  (bind _returnvalue (`GameplayStatics.SpawnEmitterAtLocation` "/Game/FluidNinja/Usecases/Particles/CollectTimeFrame.CollectTimeFrame" (`SceneComponent.K2_GetComponentLocation` (`self.Sphere`))))
  (`self.K2_DestroyActor`))

(fn `UserConstructionScript`)