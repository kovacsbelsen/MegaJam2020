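; BP_FutureSelf is an actor that stages the player's meeting with their older self, apparently as the game's ending.
; On first overlap by MainChar, the trigger starts looping animations on both characters, stops the HUD counter and disables player movement.
; After a short delay it blends in a conversation widget and enables its own input, so pressing Space quits the game.
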(event `self.PlayerTrigger.OnComponentBeginOverlap`
  (params (OverlappedComponent :type "PrimitiveComponent Object Reference") (OtherActor :type "Actor Object Reference") (OtherComp :type "PrimitiveComponent Object Reference") (OtherBodyIndex :type Integer) (bFromSweep :type Boolean) (SweepResult :type "HitResult Structure (by ref)"))
  (bind _asmain_char (cast `/Game/JamFolder/Blueprints/MainChar` OtherActor))
  (`/Engine/EditorBlueprintResources/StandardMacros.DoOnce` false
    (:`Completed`
      (`SkeletalMeshComponent.PlayAnimation` (`self.SkeletalMesh`) "/Game/Blueprints/MainCharacter/Anims/MeetingYourOldSelf_Long_Anim.MeetingYourOldSelf_Long_Anim" true)
      (`SkeletalMeshComponent.PlayAnimation` (`Character.Mesh` _asmain_char) "/Game/Blueprints/MainCharacter/Anims/ReactionToMeetingYourself_Anim.ReactionToMeetingYourself_Anim" true)
      (set `/Game/JamFolder/UI/Main_Widget.CounterOn` false (`/Game/JamFolder/Blueprints/MainChar.MainWidgetReference` _asmain_char))
      (`CharacterMovementComponent.DisableMovement` (`Character.CharacterMovement` _asmain_char))
      (`KismetSystemLibrary.Delay` 1.0)
      (bind _returnvalue (`|CreateWidget` "/Game/JamFolder/UI/Conversation_Widget.Conversation_Widget_C"))
      (bind _output_get (set `self.WidgetReference` _returnvalue))
      (`UserWidget.AddToViewport` _output_get 0)
      (`UserWidget.PlayAnimation` _returnvalue (`/Game/JamFolder/UI/Conversation_Widget.BlendIn` _returnvalue) 0.0 1 "Forward" 1.0 false)
      (`self.EnableInput` (`GameplayStatics.GetPlayerController` 0)))))

(event `Key|SpaceBar`
  (params (Key :type "Key Structure"))
  (:`Pressed`
    (`KismetSystemLibrary.QuitGame` null "Quit")))

(fn `UserConstructionScript`)