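; Coin collectible that the main character picks up by overlapping its sphere.
; On overlap it casts to MainChar, disables the sphere's collision to prevent repeat pickups, increments CoinAmount and refreshes the coin count through the character's main widget.
; It then spawns a collect particle effect, plays the pickup animation on the skeletal coin mesh and destroys itself after a short delay.
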(event `self.Sphere.OnComponentBeginOverlap`
  (params (OverlappedComponent :type "PrimitiveComponent Object Reference") (OtherActor :type "Actor Object Reference") (OtherComp :type "PrimitiveComponent Object Reference") (OtherBodyIndex :type Integer) (bFromSweep :type Boolean) (SweepResult :type "HitResult Structure (by ref)"))
  (bind _asmain_char (cast `/Game/JamFolder/Blueprints/MainChar` OtherActor))
  (`PrimitiveComponent.SetCollisionResponseToAllChannels` (`self.Sphere`) "ECR_Ignore")
  (bind _output_get (set `/Game/JamFolder/Blueprints/MainChar.CoinAmount` (+ (`/Game/JamFolder/Blueprints/MainChar.CoinAmount` _asmain_char) 1) _asmain_char))
  (`/Game/JamFolder/UI/Main_Widget.UpdateCoins` (`/Game/JamFolder/Blueprints/MainChar.MainWidgetReference` _asmain_char))
  (`GameplayStatics.SpawnEmitterAtLocation` "/Game/PlatformerDevelopmentKit/Interactables/Particles/PS_Collect.PS_Collect" (`SceneComponent.K2_GetComponentLocation` (`self.Sphere`)))
  (`SkeletalMeshComponent.PlayAnimation` (`self.SK_Coin`) "/Game/PlatformerDevelopmentKit/Interactables/Animations/CoinPickup_Anim.CoinPickup_Anim" false)
  (`KismetSystemLibrary.Delay` 1.0)
  (`self.K2_DestroyActor`))

(fn `UserConstructionScript`)