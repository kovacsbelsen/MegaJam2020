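; Overworld level-entrance base actor that shows level info while the player overlaps its sphere and loads that level on interact.
; BeginPlay builds the info widget, then fills coins, clear sign and item icons from cleared records in the game instance's LevelInfos, matched by CurrentLevel class.
; OnInteract registers or selects that record, freezes and turns the player, ground-traces to place a Hole ahead, then plays a transition before opening the level.
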(event `self.OnInteract`
  (bind _playerreference (`self.PlayerReference`))
  (bind _returnvalue (+ (`self.K2_GetActorLocation` _playerreference) (* (`KismetMathLibrary.GetForwardVector` (`self.K2_GetActorRotation` _playerreference)) 100.0)))
  (bind _leveltoload (`self.CheckLevel`))
  (`MovementComponent.StopMovementImmediately` (`Character.CharacterMovement` (`self.PlayerReference`)))
  (`self.DisableInput` (`self.PlayerReference`) (`GameplayStatics.GetPlayerController` 0))
  (`self.K2_SetActorRotation` (`self.PlayerReference`) (`KismetMathLibrary.FindLookAtRotation` (`self.K2_GetActorLocation` (`self.PlayerReference`)) (`self.K2_GetActorLocation`)) false)
  (bind _outhit (`KismetSystemLibrary.LineTraceSingle` (+ _returnvalue (0.0 0.0 200.0)) (- _returnvalue (0.0 0.0 200.0)) "TraceTypeQuery1"))
  (`SceneComponent.K2_SetWorldLocation` (`self.Hole`) (+ (`.ImpactPoint` (`GameplayStatics.BreakHitResult` _outhit)) (0.0 0.0 10.0)) false false)
  (set `/Game/JamFolder/Blueprints/MainChar.CharacterCondition` "NewEnumerator3" (`self.PlayerReference`))
  (bind _returnvalue_2 (`|CreateWidget` "/Game/PlatformerDevelopmentKit/UI/Widgets/LoadingTransition_Widget.LoadingTransition_Widget_C"))
  (`UserWidget.AddToViewport` _returnvalue_2 0)
  (bind _blendin (`/Game/PlatformerDevelopmentKit/UI/Widgets/LoadingTransition_Widget.BlendIn` _returnvalue_2))
  (`UserWidget.PlayAnimation` _returnvalue_2 _blendin 0.0 1 "Forward" 1.0 false)
  (`KismetSystemLibrary.Delay` (`WidgetAnimation.GetEndTime` _blendin))
  (`KismetSystemLibrary.Delay` 1.0)
  (`GameplayStatics.OpenLevel` _leveltoload))

(event `self.ReceiveBeginPlay`
  (bind ((`Coins_2_E21E2AA7447927285136538109124E3D` _coins) (`MainItemsAmount_8_2515D8D640D75E707030479E148218E8` _mainitemsamount) (`MainItemsHighscoreAmount_63_A1BADD1A4DF3EEECAA6A10BC1EA22917` _mainitemshighscoreamount) (`CurrentLevel_33_30F5522E43C6F1C9CEB164B0C3D8874B` _currentlevel) (`LevelCleared?_26_839792B648B06B5E5B491FB8A864C38B` _levelcleared_) (`MainItemIcon_29_432831BB429E7639BB624A90C8ED4743` _mainitemicon) (`LevelName_40_46E954964AF076BA87A0AD9AD6DC0735` _levelname) (`LevelToLoad_43_2A6201CD41C6179B389CBFBD0A779DE5` _leveltoload) (`MainItems_50_89FB1DA64E49B059B81CEF9F5A237C16` _mainitems) (`LevelInfoWidget_54_0251784745817F6072098385EC916917` _levelinfowidget)) (break `/Game/PlatformerDevelopmentKit/Overworld/Blueprints/S_Levelvariables` (`self.LevelVariables`)))
  (bind (_coins_2 _mainitemsamount_2 _mainitemshighscoreamount_2 _currentlevel_2 _levelcleared__2 _mainitemicon_2 _levelname_2 _leveltoload_2 _gameinstance _mainitems_2) (break `/Game/PlatformerDevelopmentKit/Overworld/Blueprints/S_Levelvariables` (`self.LevelVariables`)))
  (bind (_coins_3 _mainitemsamount_3 _mainitemshighscoreamount_3 _currentlevel_3 _levelcleared__3 _mainitemicon_3 _levelname_3 _leveltoload_3 _gameinstance_2 _mainitems_3 _levelinfowidget_2) (break `/Game/PlatformerDevelopmentKit/Overworld/Blueprints/S_Levelvariables` (`self.LevelVariables`)))
  (bind _asbp_platformer_game_instance (cast `/Game/PlatformerDevelopmentKit/Base/Blueprints/BP_PlatformerGameInstance` (`GameplayStatics.GetGameInstance`)))
  (set `self.LevelVariables` (make `/Game/PlatformerDevelopmentKit/Overworld/Blueprints/S_Levelvariables` _coins_3 _mainitemsamount_3 _mainitemshighscoreamount_3 _currentlevel_3 _levelcleared__3 _mainitemicon_3 _levelname_3 _leveltoload_3 _asbp_platformer_game_instance _mainitems_3 _levelinfowidget_2))
  (bind _aslevel_info_widget (cast `/Game/PlatformerDevelopmentKit/Overworld/Widgets/LevelInfo_Widget` (`WidgetComponent.GetUserWidgetObject` (`self.LevelInfo`))))
  (set `self.LevelVariables` (make `/Game/PlatformerDevelopmentKit/Overworld/Blueprints/S_Levelvariables` _coins_2 _mainitemsamount_2 _mainitemshighscoreamount_2 _currentlevel_2 _levelcleared__2 _mainitemicon_2 _levelname_2 _leveltoload_2 _gameinstance _mainitems_2 _aslevel_info_widget))
  (`TextBlock.SetText` (`/Game/PlatformerDevelopmentKit/Overworld/Widgets/LevelInfo_Widget.LevelName` _levelinfowidget) _levelname)
  (for _ (range 1 (+ _mainitemsamount 1))
    (bind _returnvalue (`|CreateWidget` "/Game/PlatformerDevelopmentKit/Overworld/Widgets/LevelMainItem_Widget.LevelMainItem_Widget_C"))
    (`HorizontalBox.AddChildToHorizontalBox` (`/Game/PlatformerDevelopmentKit/Overworld/Widgets/LevelInfo_Widget.MainItemBox` _levelinfowidget) _returnvalue)
    (`KismetArrayLibrary.Array_Add` _mainitems _returnvalue))
  (`self.UpdateLevelInfo`))

(event `self.Sphere.OnComponentBeginOverlap`
  (params (OverlappedComponent :type "PrimitiveComponent Object Reference") (OtherActor :type "Actor Object Reference") (OtherComp :type "PrimitiveComponent Object Reference") (OtherBodyIndex :type Integer) (bFromSweep :type Boolean) (SweepResult :type "HitResult Structure (by ref)"))
  (bind _asmain_char (cast `/Game/JamFolder/Blueprints/MainChar` OtherActor))
  (set `self.PlayerReference` _asmain_char)
  (`SceneComponent.SetVisibility` (`self.LevelInfo`) true false))

(event `self.Sphere.OnComponentEndOverlap`
  (params (OverlappedComponent :type "PrimitiveComponent Object Reference") (OtherActor :type "Actor Object Reference") (OtherComp :type "PrimitiveComponent Object Reference") (OtherBodyIndex :type Integer))
  (bind _asmain_char (cast `/Game/JamFolder/Blueprints/MainChar` OtherActor))
  (set `self.PlayerReference` _asmain_char)
  (`SceneComponent.SetVisibility` (`self.LevelInfo`) false false))

(fn `CheckLevel`
  (returns (LevelToLoad :type Name))
  (locals (`FoundSameLevel?` :type Boolean))
  (bind (_coins _mainitemsamount _mainitemshighscoreamount _currentlevel _levelcleared_ _mainitemicon _levelname _leveltoload _gameinstance) (break `/Game/PlatformerDevelopmentKit/Overworld/Blueprints/S_Levelvariables` (`self.LevelVariables`)))
  (bind _levelinfos (`/Game/PlatformerDevelopmentKit/Base/Blueprints/BP_PlatformerGameInstance.LevelInfos` (`.GameInstance_46_9F3790CC4508A67A61D37F9BDF8933B8` (break `/Game/PlatformerDevelopmentKit/Overworld/Blueprints/S_Levelvariables` (`self.LevelVariables`)))))
  (if (`KismetArrayLibrary.Array_IsValidIndex` _levelinfos)
    (for (_array_element _array_index) _levelinfos
      (if (== (`.CurrentLevel_33_30F5522E43C6F1C9CEB164B0C3D8874B` (break `/Game/PlatformerDevelopmentKit/Overworld/Blueprints/S_Levelvariables` _array_element)) (`.CurrentLevel_33_30F5522E43C6F1C9CEB164B0C3D8874B` (break `/Game/PlatformerDevelopmentKit/Overworld/Blueprints/S_Levelvariables` (`self.LevelVariables`))))
        (set `local.FoundSameLevel?` true)
        (set `/Game/PlatformerDevelopmentKit/Base/Blueprints/BP_PlatformerGameInstance.CurrentLevelIndex` _array_index _gameinstance)
        (break))))
  (if (`local.FoundSameLevel?`)
    (return _leveltoload)
    (else
      (bind _returnvalue (`KismetArrayLibrary.Array_Add` (`/Game/PlatformerDevelopmentKit/Base/Blueprints/BP_PlatformerGameInstance.LevelInfos` _gameinstance) (`self.LevelVariables`)))
      (set `/Game/PlatformerDevelopmentKit/Base/Blueprints/BP_PlatformerGameInstance.CurrentLevelIndex` _returnvalue _gameinstance)
      (return _leveltoload))))

(fn `UpdateLevelInfo`
  (locals (LocalLevelInfo :type "/Game/PlatformerDevelopmentKit/Overworld/Blueprints/S_Levelvariables Structure"))
  (bind (_coins _mainitemsamount _mainitemshighscoreamount _currentlevel _levelcleared_ _mainitemicon) (break `/Game/PlatformerDevelopmentKit/Overworld/Blueprints/S_Levelvariables` (`local.LocalLevelInfo`)))
  (for _array_element (`/Game/PlatformerDevelopmentKit/Base/Blueprints/BP_PlatformerGameInstance.LevelInfos` (`.GameInstance_46_9F3790CC4508A67A61D37F9BDF8933B8` (break `/Game/PlatformerDevelopmentKit/Overworld/Blueprints/S_Levelvariables` (`self.LevelVariables`))))
    (bind (_coins_2 _mainitemsamount_2 _mainitemshighscoreamount_2 _currentlevel_2 _levelcleared__2) (break `/Game/PlatformerDevelopmentKit/Overworld/Blueprints/S_Levelvariables` _array_element))
    (if (== _currentlevel_2 (`.CurrentLevel_33_30F5522E43C6F1C9CEB164B0C3D8874B` (break `/Game/PlatformerDevelopmentKit/Overworld/Blueprints/S_Levelvariables` (`self.LevelVariables`))))
      (if _levelcleared__2
        (set `local.LocalLevelInfo` _array_element)
        (bind _outactors (`GameplayStatics.GetAllActorsOfClass` _currentlevel))
        (for _array_element_2 _outactors
          (bind (_coins_3 _mainitemsamount_3 _mainitemshighscoreamount_3 _currentlevel_3 _levelcleared__3 _mainitemicon_2 _levelname _leveltoload _gameinstance _mainitems _levelinfowidget) (break `/Game/PlatformerDevelopmentKit/Overworld/Blueprints/S_Levelvariables` (`/Game/PlatformerDevelopmentKit/Overworld/Blueprints/BP_OverworldLevelMaster.LevelVariables` _array_element_2)))
          (`TextBlock.SetText` (`/Game/PlatformerDevelopmentKit/Overworld/Widgets/LevelInfo_Widget.CoinAmount` _levelinfowidget) (`KismetTextLibrary.Conv_IntToText` _coins))
          (`Widget.SetVisibility` (`/Game/PlatformerDevelopmentKit/Overworld/Widgets/LevelInfo_Widget.ClearSign` _levelinfowidget) "Visible")
          (for _ (range 1 (+ _mainitemshighscoreamount 1))
            (for _array_element_3 _mainitems
              (if (`/Game/PlatformerDevelopmentKit/Overworld/Widgets/LevelMainItem_Widget.IsEmpty?` _array_element_3)
                (`Image.SetBrushFromTexture` (`/Game/PlatformerDevelopmentKit/Overworld/Widgets/LevelMainItem_Widget.Icon` _array_element_3) _mainitemicon false)
                (set `/Game/PlatformerDevelopmentKit/Overworld/Widgets/LevelMainItem_Widget.IsEmpty?` false _array_element_3)
                (break)))))))))

(fn `UserConstructionScript`)