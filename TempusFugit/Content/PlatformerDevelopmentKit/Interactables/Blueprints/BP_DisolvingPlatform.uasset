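; A dissolving platform that falls away after the player character steps on it, then returns.
; An overlap with the Box1 trigger by MainChar fires once, playing the consume animation on the skeletal platform.
; After a delay, Box ignores collision and the platform hides.
; After a second delay it reappears with a spawn animation, blocks again and re-arms the trigger.
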(event `self.Box1.OnComponentBeginOverlap`
  (params (OverlappedComponent :type "PrimitiveComponent Object Reference") (OtherActor :type "Actor Object Reference") (OtherComp :type "PrimitiveComponent Object Reference") (OtherBodyIndex :type Integer) (bFromSweep :type Boolean) (SweepResult :type "HitResult Structure (by ref)"))
  (bind _sk_platform (`self.SK_Platform`))
  (bind _asmain_char (cast `/Game/JamFolder/Blueprints/MainChar` OtherActor))
  (`/Engine/EditorBlueprintResources/StandardMacros.DoOnce` false :!label _label
    (:`Completed`
      (set `self.PlayerReference` _asmain_char)
      (`SkeletalMeshComponent.PlayAnimation` (`self.SK_Platform`) "/Game/PlatformerDevelopmentKit/Interactables/Animations/ConsumePlatform_Anim.ConsumePlatform_Anim" false)
      (`KismetSystemLibrary.Delay` 7.0)
      (`PrimitiveComponent.SetCollisionResponseToAllChannels` (`self.Box`) "ECR_Ignore")
      (`SceneComponent.SetVisibility` (`self.SK_Platform`) false false)
      (`KismetSystemLibrary.Delay` 7.0)
      (`SceneComponent.SetVisibility` _sk_platform true false)
      (`SkeletalMeshComponent.PlayAnimation` _sk_platform "/Game/PlatformerDevelopmentKit/Interactables/Animations/SpawnPlatform_Anim.SpawnPlatform_Anim" false)
      (`PrimitiveComponent.SetCollisionResponseToAllChannels` (`self.Box`) "ECR_Block")
      (goto _label :!via `Reset`))))

(fn `UserConstructionScript`)