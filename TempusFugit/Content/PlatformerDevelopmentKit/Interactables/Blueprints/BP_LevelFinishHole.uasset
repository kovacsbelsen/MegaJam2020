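; Level-end goal hole that finishes the level when the MainChar overlaps its sphere.
; It freezes the player, snaps them to traced ground facing the hole, then shows a finish screen with coins and found versus total MainItems.
; After a loading transition, it writes beaten coin or item records and LevelCleared to the GameInstance, flags a save prompt and opens the overworld.
; ItemCounter holds the level total, then is reused for the collected count.
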(event `self.ReceiveBeginPlay`
  (bind _outactors (`GameplayStatics.GetAllActorsOfClass` (`self.MainItem`)))
  (for _ _outactors
    (set `self.ItemCounter` (+ (`self.ItemCounter`) 1))))

(event `self.Sphere.OnComponentBeginOverlap`
  (params (OverlappedComponent :type "PrimitiveComponent Object Reference") (OtherActor :type "Actor Object Reference") (OtherComp :type "PrimitiveComponent Object Reference") (OtherBodyIndex :type Integer) (bFromSweep :type Boolean) (SweepResult :type "HitResult Structure (by ref)"))
  (bind _finishscreenreference (`self.FinishScreenReference`))
  (bind _playerreference (`self.PlayerReference`))
  (bind _gameinstance (`self.GameInstance`))
  (bind _gameinstance_2 (`self.GameInstance`))
  (bind _gameinstance_3 (`self.GameInstance`))
  (bind _playerreference_2 (`self.PlayerReference`))
  (bind _returnvalue (`SceneComponent.K2_GetComponentLocation` (`self.Arrow1`)))
  (bind _coinamount (`/Game/JamFolder/Blueprints/MainChar.CoinAmount` (`self.PlayerReference`)))
  (bind _finishscreenblendin (`/Game/PlatformerDevelopmentKit/UI/Widgets/FinishScreen_Widget.FinishScreenBlendIn` _finishscreenreference))
  (bind (_coins _mainitemsamount _mainitemshighscoreamount _currentlevel _levelcleared_ _mainitemicon _levelname _leveltoload _gameinstance_4 _mainitems _levelinfowidget) (break `/Game/PlatformerDevelopmentKit/Overworld/Blueprints/S_Levelvariables` (`|GetArrayItem` (`/Game/PlatformerDevelopmentKit/Base/Blueprints/BP_PlatformerGameInstance.LevelInfos` _gameinstance_3) (`/Game/PlatformerDevelopmentKit/Base/Blueprints/BP_PlatformerGameInstance.CurrentLevelIndex` _gameinstance_3))))
  (bind _asmain_char (cast `/Game/JamFolder/Blueprints/MainChar` OtherActor))
  (set `self.PlayerReference` _asmain_char)
  (`SceneComponent.K2_SetWorldRotation` (`self.Arrow`) (`KismetMathLibrary.MakeRotator` 0.0 0.0 (.yaw (`KismetMathLibrary.FindLookAtRotation` (`SceneComponent.K2_GetComponentLocation` (`self.Arrow`)) (`self.K2_GetActorLocation` (`self.PlayerReference`))))) false false)
  (`MovementComponent.StopMovementImmediately` (`Character.CharacterMovement` _playerreference_2))
  (`self.DisableInput` _playerreference_2 (`GameplayStatics.GetPlayerController` 0))
  (bind _outhit (`KismetSystemLibrary.LineTraceSingle` _returnvalue (- _returnvalue (0.0 0.0 1000.0)) "TraceTypeQuery1"))
  (`self.K2_SetActorLocation` (`self.PlayerReference`) (+ (`.ImpactPoint` (`GameplayStatics.BreakHitResult` _outhit)) (`KismetMathLibrary.MakeVector` 0.0 0.0 (`CapsuleComponent.CapsuleHalfHeight` (`Character.CapsuleComponent` (`self.PlayerReference`))))) false true)
  (`self.K2_SetActorRotation` _playerreference (`KismetMathLibrary.MakeRotator` 0.0 0.0 (.yaw (`KismetMathLibrary.FindLookAtRotation` (`self.K2_GetActorLocation` (`self.PlayerReference`)) (`self.K2_GetActorLocation`)))) false)
  (set `/Game/JamFolder/Blueprints/MainChar.CharacterCondition` "NewEnumerator3" _playerreference)
  (`KismetSystemLibrary.Delay` 1.0)
  (bind _returnvalue_2 (`|CreateWidget` "/Game/PlatformerDevelopmentKit/UI/Widgets/FinishScreen_Widget.FinishScreen_Widget_C"))
  (set `self.FinishScreenReference` _returnvalue_2)
  (`self.SetFinishScreen`)
  (`UserWidget.AddToViewport` _returnvalue_2 0)
  (`UserWidget.PlayAnimation` _finishscreenreference _finishscreenblendin 0.0 1 "Forward" 1.0 false)
  (`KismetSystemLibrary.Delay` (`WidgetAnimation.GetEndTime` _finishscreenblendin))
  (`KismetSystemLibrary.Delay` 5.0)
  (bind _returnvalue_3 (`|CreateWidget` "/Game/PlatformerDevelopmentKit/UI/Widgets/LoadingTransition_Widget.LoadingTransition_Widget_C"))
  (`UserWidget.AddToViewport` _returnvalue_3 0)
  (bind _blendin (`/Game/PlatformerDevelopmentKit/UI/Widgets/LoadingTransition_Widget.BlendIn` _returnvalue_3))
  (`UserWidget.PlayAnimation` _returnvalue_3 _blendin 0.0 1 "Forward" 1.0 false)
  (`KismetSystemLibrary.Delay` (`WidgetAnimation.GetEndTime` _blendin))
  (`KismetSystemLibrary.Delay` 1.0)
  (bind _asbp_platformer_game_instance (cast `/Game/PlatformerDevelopmentKit/Base/Blueprints/BP_PlatformerGameInstance` (`GameplayStatics.GetGameInstance`)))
  (bind _output_get (set `self.GameInstance` _asbp_platformer_game_instance))
  (bind (_coins_2 _mainitemsamount_2 _mainitemshighscoreamount_2 _currentlevel_2 _levelcleared__2 _mainitemicon_2 _levelname_2 _leveltoload_2 _gameinstance_5 _mainitems_2 _levelinfowidget_2) (break `/Game/PlatformerDevelopmentKit/Overworld/Blueprints/S_Levelvariables` (`|GetArrayItem` (`/Game/PlatformerDevelopmentKit/Base/Blueprints/BP_PlatformerGameInstance.LevelInfos` _output_get) (`/Game/PlatformerDevelopmentKit/Base/Blueprints/BP_PlatformerGameInstance.CurrentLevelIndex` _output_get))))
  (if (> _coinamount _coins_2)
    (`KismetArrayLibrary.Array_Set` (`/Game/PlatformerDevelopmentKit/Base/Blueprints/BP_PlatformerGameInstance.LevelInfos` _gameinstance_2) (`/Game/PlatformerDevelopmentKit/Base/Blueprints/BP_PlatformerGameInstance.CurrentLevelIndex` _gameinstance_2) (make `/Game/PlatformerDevelopmentKit/Overworld/Blueprints/S_Levelvariables` _coinamount _mainitemsamount_2 _mainitemshighscoreamount_2 _currentlevel_2 true _mainitemicon_2 _levelname_2 _leveltoload_2 _gameinstance_5 _mainitems_2 _levelinfowidget_2)))
  (if (> (`self.ItemCounter`) _mainitemshighscoreamount)
    (`KismetArrayLibrary.Array_Set` (`/Game/PlatformerDevelopmentKit/Base/Blueprints/BP_PlatformerGameInstance.LevelInfos` _gameinstance) (`/Game/PlatformerDevelopmentKit/Base/Blueprints/BP_PlatformerGameInstance.CurrentLevelIndex` _gameinstance) (make `/Game/PlatformerDevelopmentKit/Overworld/Blueprints/S_Levelvariables` _coins _mainitemsamount (`self.ItemCounter`) _currentlevel true (`.Icon_2_032777E34EFD0271F978D98F441B05EA` (break `/Game/PlatformerDevelopmentKit/Base/Blueprints/S_ItemInfo` (`.ItemInfo` (defaults `Object` (`self.MainItem`))))) _levelname _leveltoload _gameinstance_4 _mainitems _levelinfowidget)))
  (set `/Game/PlatformerDevelopmentKit/Base/Blueprints/BP_PlatformerGameInstance.PromotSave?` true (`self.GameInstance`))
  (`GameplayStatics.OpenLevel` "Map_Overworld"))

(fn `CheckHighscore`
  (returns (LastMainItemHighscore :type Integer) (LastCoinAmountHighscore :type Integer))
  (locals (NotEmptyCounter :type Integer))
  (bind _gameinstance (`self.GameInstance`))
  (bind (_coins _mainitemsamount _mainitemshighscoreamount _currentlevel _levelcleared_ _mainitemicon _levelname _leveltoload _gameinstance_2 _mainitems) (break `/Game/PlatformerDevelopmentKit/Overworld/Blueprints/S_Levelvariables` (`|GetArrayItem` (`/Game/PlatformerDevelopmentKit/Base/Blueprints/BP_PlatformerGameInstance.LevelInfos` _gameinstance) (`/Game/PlatformerDevelopmentKit/Base/Blueprints/BP_PlatformerGameInstance.CurrentLevelIndex` _gameinstance))))
  (for _array_element _mainitems
    (if (not (`/Game/PlatformerDevelopmentKit/Overworld/Widgets/LevelMainItem_Widget.IsEmpty?` _array_element))
      (`/Engine/EditorBlueprintResources/StandardMacros.IncrementInt` (`local.NotEmptyCounter`))))
  (return (`local.NotEmptyCounter`) _coins))

(fn `SetFinishScreen`
  (`TextBlock.SetText` (`/Game/PlatformerDevelopmentKit/UI/Widgets/FinishScreen_Widget.CoinAmount` (`self.FinishScreenReference`)) (`KismetTextLibrary.Conv_IntToText` (`/Game/JamFolder/Blueprints/MainChar.CoinAmount` (`self.PlayerReference`))))
  (`TextBlock.SetText` (`/Game/PlatformerDevelopmentKit/UI/Widgets/FinishScreen_Widget.AmountFoundInLevel` (`self.FinishScreenReference`)) (`KismetTextLibrary.Conv_IntToText` (`self.ItemCounter`)))
  (set `self.ItemCounter` 0)
  (for _array_element (`/Game/JamFolder/Blueprints/MainChar.CollectedItems` (`self.PlayerReference`))
    (if (== _array_element (`self.MainItem`))
      (set `self.ItemCounter` (+ (`self.ItemCounter`) 1))
      (bind _returnvalue (`|CreateWidget` "/Game/PlatformerDevelopmentKit/UI/Widgets/FinishScreenItem_Widget.FinishScreenItem_Widget_C"))
      (`Image.SetBrushFromTexture` (`/Game/PlatformerDevelopmentKit/UI/Widgets/FinishScreenItem_Widget.ItemIcon` _returnvalue) (`.Icon_2_032777E34EFD0271F978D98F441B05EA` (break `/Game/PlatformerDevelopmentKit/Base/Blueprints/S_ItemInfo` (`.ItemInfo` (defaults `Object` (`self.MainItem`))))) false)
      (`HorizontalBox.AddChildToHorizontalBox` (`/Game/PlatformerDevelopmentKit/UI/Widgets/FinishScreen_Widget.CollectedItemsBox` (`self.FinishScreenReference`)) _returnvalue)
      (`Widget.SetRenderTransform` _returnvalue (make `WidgetTransform` (`KismetMathLibrary.MakeVector2D` 0.0 (`KismetMathLibrary.RandomFloatInRange` -40.0 10.0)) (1.0 1.0) (0.0 0.0) (`KismetMathLibrary.RandomFloatInRange` -10.0 10.0)))))
  (`TextBlock.SetText` (`/Game/PlatformerDevelopmentKit/UI/Widgets/FinishScreen_Widget.AmountCollected` (`self.FinishScreenReference`)) (`KismetTextLibrary.Conv_IntToText` (`self.ItemCounter`))))

(fn `UserConstructionScript`)