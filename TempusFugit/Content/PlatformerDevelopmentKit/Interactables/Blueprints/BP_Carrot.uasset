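; BP_Carrot is a pickup that updates the player's hearts by one when MainChar overlaps its sphere.
; On overlap it sets the sphere to ignore all collision, preventing repeat triggers, and calls UpdateHearts on the character's main widget.
; It then spawns a crumb particle effect, plays the skeletal carrot's pickup animation, and destroys itself after a short fixed delay.
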(event `self.Sphere.OnComponentBeginOverlap`
  (params (OverlappedComponent :type "PrimitiveComponent Object Reference") (OtherActor :type "Actor Object Reference") (OtherComp :type "PrimitiveComponent Object Reference") (OtherBodyIndex :type Integer) (bFromSweep :type Boolean) (SweepResult :type "HitResult Structure (by ref)"))
  (bind _asmain_char (cast `/Game/JamFolder/Blueprints/MainChar` OtherActor))
  (`PrimitiveComponent.SetCollisionResponseToAllChannels` (`self.Sphere`) "ECR_Ignore")
  (`/Game/JamFolder/UI/Main_Widget.UpdateHearts` (`/Game/JamFolder/Blueprints/MainChar.MainWidgetReference` _asmain_char) 1)
  (`GameplayStatics.SpawnEmitterAtLocation` "/Game/PlatformerDevelopmentKit/Interactables/Particles/PS_CarrotCrums.PS_CarrotCrums" (`SceneComponent.K2_GetComponentLocation` (`self.Sphere`)))
  (`SkeletalMeshComponent.PlayAnimation` (`self.SK_Carrot`) "/Game/PlatformerDevelopmentKit/Interactables/Animations/CarrotPickup_Anim.CarrotPickup_Anim" false)
  (`KismetSystemLibrary.Delay` 0.583)
  (`self.K2_DestroyActor`))

(fn `UserConstructionScript`)