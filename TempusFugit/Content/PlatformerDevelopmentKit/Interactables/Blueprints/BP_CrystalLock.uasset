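; A crystal lock interactable that shatters when the player touches it while carrying the required item.
; BeginPlay puts the required item's icon into a lock widget, hidden when ShowRequiredItem is off.
; Sphere overlap passes through a gate, then consumes the matching item from MainChar's CollectedItems and HUD.
; On success it damages the destructible crystal, disables its collision, closes the gate, clears the icon and destroys itself after a delay.
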(event `self.ReceiveBeginPlay`
  (if (not (`self.ShowRequiredItem?`))
    (`SceneComponent.SetVisibility` (`self.RequiredItemWidget`) false false))
  (bind _returnvalue (`|CreateWidget` "/Game/PlatformerDevelopmentKit/UI/Widgets/Item_Widget.Item_Widget_C"))
  (`Image.SetBrushFromTexture` (`/Game/PlatformerDevelopmentKit/UI/Widgets/Item_Widget.ItemIcon` _returnvalue) (`.Icon_2_032777E34EFD0271F978D98F441B05EA` (break `/Game/PlatformerDevelopmentKit/Base/Blueprints/S_ItemInfo` (`.ItemInfo` (defaults `Object` (`self.RequiredItem`))))) false)
  (bind _aslock_item_widget (cast `/Game/PlatformerDevelopmentKit/UI/Widgets/LockItem_Widget` (`WidgetComponent.GetUserWidgetObject` (`self.RequiredItemWidget`))))
  (set `self.RequiredItemWidgetReference` _aslock_item_widget)
  (`PanelWidget.AddChild` (`/Game/PlatformerDevelopmentKit/UI/Widgets/LockItem_Widget.ItemRequired` _aslock_item_widget) _returnvalue))

(event `LockFurtherInteraction`
  (bind _ad_crystal (`self.AD_Crystal`))
  (bind _returnvalue (`SceneComponent.K2_GetComponentLocation` _ad_crystal))
  (goto _label :!via `Close`))

(event `self.Sphere.OnComponentBeginOverlap`
  (params (OverlappedComponent :type "PrimitiveComponent Object Reference") (OtherActor :type "Actor Object Reference") (OtherComp :type "PrimitiveComponent Object Reference") (OtherBodyIndex :type Integer) (bFromSweep :type Boolean) (SweepResult :type "HitResult Structure (by ref)"))
  (bind _ad_crystal (`self.AD_Crystal`))
  (bind _returnvalue (`SceneComponent.K2_GetComponentLocation` _ad_crystal))
  (`/Engine/EditorBlueprintResources/StandardMacros.Gate` false :!label _label
    (:`Exit`
      (bind _asmain_char (cast `/Game/JamFolder/Blueprints/MainChar` OtherActor))
      (set `self.PlayerReference` _asmain_char)
      (bind _playerhasitemrequired_ (`self.CheckIfPlayerHasRequiredItem`))
      (if _playerhasitemrequired_
        (`GameplayStatics.ApplyDamage` _ad_crystal null 0.0 null null null 1.0 _returnvalue _returnvalue)
        (`PrimitiveComponent.SetCollisionResponseToAllChannels` (`self.AD_Crystal`) "ECR_Ignore")
        (`self.LockFurtherInteraction`)
        (`PanelWidget.ClearChildren` (`/Game/PlatformerDevelopmentKit/UI/Widgets/LockItem_Widget.ItemRequired` (`self.RequiredItemWidgetReference`)))
        (`KismetSystemLibrary.Delay` 10.0)
        (`self.K2_DestroyActor`)))))

(event `self.Sphere.OnComponentEndOverlap`
  (params (OverlappedComponent :type "PrimitiveComponent Object Reference") (OtherActor :type "Actor Object Reference") (OtherComp :type "PrimitiveComponent Object Reference") (OtherBodyIndex :type Integer)))

(fn `CheckIfPlayerHasRequiredItem`
  (returns (`PlayerHasItemRequired?` :type Boolean))
  (locals (`FoundItem?` :type Boolean))
  (for (_array_element _array_index) (`/Game/JamFolder/Blueprints/MainChar.CollectedItems` (`self.PlayerReference`))
    (if (== _array_element (`self.RequiredItem`))
      (set `local.FoundItem?` true)
      (`KismetArrayLibrary.Array_Remove` (`/Game/JamFolder/Blueprints/MainChar.CollectedItems` (`self.PlayerReference`)) _array_index)
      (break)
      (else
        (set `local.FoundItem?` false))))
  (if (`local.FoundItem?`)
    (for _array_element_2 (`/Game/PlatformerDevelopmentKit/UI/Widgets/Main_Widget.ItemWidgets` (`/Game/JamFolder/Blueprints/MainChar.MainWidgetReference` (`self.PlayerReference`)))
      (if (== (`.Class_5_1A8C90744C7F5319380E0C8DD249B8CE` (break `/Game/PlatformerDevelopmentKit/Base/Blueprints/S_ItemInfo` (`/Game/PlatformerDevelopmentKit/UI/Widgets/Item_Widget.ItemInfo` _array_element_2))) (`self.RequiredItem`))
        (`Widget.RemoveFromParent` _array_element_2)
        (break)))
    (return true)
    (else
      (return false))))

(fn `UserConstructionScript`)