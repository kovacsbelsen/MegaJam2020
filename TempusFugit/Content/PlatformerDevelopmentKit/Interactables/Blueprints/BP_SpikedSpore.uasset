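; Spiked spore hazard that knocks back and damages the MainChar player on touching its sphere.
; A hit drops the player from any ledge, disables input, launches them backward and upward, changes their condition, spawns an impact effect and removes a heart.
; Zero health sets a different condition.
; A DoOnce gate limits repeat hits, reset after a short delay through CanBeDamagedAgain.
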(event `CanBeDamagedAgain`
  (bind _playerreference (`self.PlayerReference`))
  (bind _playerreference_2 (`self.PlayerReference`))
  (bind (_returnvalue_x _returnvalue_y) (`KismetMathLibrary.BreakVector` (`self.GetActorForwardVector` (`self.PlayerReference`))))
  (goto _label :!via `Reset`))

(event `self.Sphere.OnComponentBeginOverlap`
  (params (OverlappedComponent :type "PrimitiveComponent Object Reference") (OtherActor :type "Actor Object Reference") (OtherComp :type "PrimitiveComponent Object Reference") (OtherBodyIndex :type Integer) (bFromSweep :type Boolean) (SweepResult :type "HitResult Structure (by ref)"))
  (bind _playerreference (`self.PlayerReference`))
  (bind _playerreference_2 (`self.PlayerReference`))
  (bind (_returnvalue_x _returnvalue_y) (`KismetMathLibrary.BreakVector` (`self.GetActorForwardVector` (`self.PlayerReference`))))
  (bind _asmain_char (cast `/Game/JamFolder/Blueprints/MainChar` OtherActor))
  (bind _output_get (set `self.PlayerReference` _asmain_char))
  (`/Engine/EditorBlueprintResources/StandardMacros.DoOnce` false :!label _label
    (:`Completed`
      (if (`/Game/JamFolder/Blueprints/MainChar.IsHanging?` (`self.PlayerReference`))
        (`/Game/JamFolder/Blueprints/MainChar.GetOffLedge` (`self.PlayerReference`)))
      (`self.DisableInput` _output_get (`GameplayStatics.GetPlayerController` 0))
      (`Character.LaunchCharacter` _playerreference (`KismetMathLibrary.MakeVector` (* _returnvalue_x -500.0) (* _returnvalue_y -500.0) 300.0) true true)
      (set `/Game/JamFolder/Blueprints/MainChar.CharacterCondition` "NewEnumerator0" _playerreference)
      (`GameplayStatics.SpawnEmitterAtLocation` "/Game/PlatformerDevelopmentKit/Characters/Player/Particles/PS_Impact.PS_Impact" (`self.K2_GetActorLocation` _playerreference))
      (`/Game/JamFolder/UI/Main_Widget.UpdateHearts` (`/Game/JamFolder/Blueprints/MainChar.MainWidgetReference` (`self.PlayerReference`)) -1)
      (if (<= (`/Game/JamFolder/Blueprints/MainChar.CurrentHealth` (`self.PlayerReference`)) 0)
        (set `/Game/JamFolder/Blueprints/MainChar.CharacterCondition` "NewEnumerator1" _playerreference_2)
        (`self.DisableInput` _playerreference_2 (`GameplayStatics.GetPlayerController` 0))
        (`KismetSystemLibrary.Delay` 0.5)
        (`self.CanBeDamagedAgain`)
        (else
          (`KismetSystemLibrary.Delay` 0.5)
          (`self.CanBeDamagedAgain`))))))

(fn `UserConstructionScript`)