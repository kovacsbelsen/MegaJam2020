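; BP_Life is an extra-life pickup in the platformer kit.
; When MainChar overlaps its sphere, it disables the sphere's collision, increments the player's Lives and refreshes the lives display on the main widget.
; It then spawns a collect particle effect, plays a pickup animation on its skeletal mesh, and destroys itself after a short delay.
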(event `self.Sphere.OnComponentBeginOverlap`
  (params (OverlappedComponent :type "PrimitiveComponent Object Reference") (OtherActor :type "Actor Object Reference") (OtherComp :type "PrimitiveComponent Object Reference") (OtherBodyIndex :type Integer) (bFromSweep :type Boolean) (SweepResult :type "HitResult Structure (by ref)"))
  (bind _asbp_rabbit (cast `/Game/JamFolder/Blueprints/MainChar` OtherActor))
  (`PrimitiveComponent.SetCollisionResponseToAllChannels` (`self.Sphere`) "ECR_Ignore")
  (set `/Game/JamFolder/Blueprints/MainChar.Lives` (+ (`/Game/JamFolder/Blueprints/MainChar.Lives` _asbp_rabbit) 1) _asbp_rabbit)
  (`/Game/PlatformerDevelopmentKit/UI/Widgets/Main_Widget.UpdateLives` (`/Game/JamFolder/Blueprints/MainChar.MainWidgetReference` _asbp_rabbit))
  (`GameplayStatics.SpawnEmitterAtLocation` "/Game/PlatformerDevelopmentKit/Interactables/Particles/PS_Collect.PS_Collect" (`SceneComponent.K2_GetComponentLocation` (`self.Sphere`)))
  (`SkeletalMeshComponent.PlayAnimation` (`self.SK_Life`) "/Game/PlatformerDevelopmentKit/Interactables/Animations/StarPickup_Anim.StarPickup_Anim" false)
  (`KismetSystemLibrary.Delay` 1.0)
  (`self.K2_DestroyActor`))

(fn `UserConstructionScript`)