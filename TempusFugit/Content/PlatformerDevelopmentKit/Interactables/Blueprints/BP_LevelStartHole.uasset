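; BP_LevelStartHole is the level's entry point, spawning and initializing the player character when play begins.
; It traces down from SpawnLocation to place MainChar above the ground, sets health and lives, hands it a self-reference, disables input and faces it away from the hole.
; A loading blend-out widget plays, then after a delay the game instance's PromotSave flag decides whether a save window opens with the mouse cursor.
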(event `self.ReceiveBeginPlay`
  (bind _returnvalue (`GameplayStatics.GetPlayerController` 0))
  (bind _playerreference (`self.PlayerReference`))
  (bind _returnvalue_2 (`SceneComponent.K2_GetComponentLocation` (`self.SpawnLocation`)))
  (bind _outhit (`KismetSystemLibrary.LineTraceSingle` _returnvalue_2 (- _returnvalue_2 (0.0 0.0 2000.0)) "TraceTypeQuery1"))
  (bind _returnvalue_3 (`|SpawnActorFromClass` "/Game/JamFolder/Blueprints/MainChar.MainChar_C" (`KismetMathLibrary.MakeTransform` (+ (`.ImpactPoint` (`GameplayStatics.BreakHitResult` _outhit)) (0.0 0.0 65.0))) "Undefined" "OverrideRootScale" null null))
  (set `self.PlayerReference` _returnvalue_3)
  (bind _returnvalue_4 (`GameplayStatics.GetCurrentLevelName` true))
  (if (`KismetStringLibrary.EqualEqual_StrStr` _returnvalue_4 (`self.OverworldLevelName`))
    _
    (else
      _))
  (set `/Game/JamFolder/Blueprints/MainChar.CurrentHealth` (`self.SerHeartsAmount`) _playerreference)
  (set `/Game/JamFolder/Blueprints/MainChar.Lives` (`self.SetLivesAmount`) _playerreference)
  (set `/Game/JamFolder/Blueprints/MainChar.StartHoleReference` self (`self.PlayerReference`))
  (`self.DisableInput` (`self.PlayerReference`) (`GameplayStatics.GetPlayerController` 0))
  (bind _returnvalue_5 (`|CreateWidget` "/Game/PlatformerDevelopmentKit/UI/Widgets/LoadingTransition_Widget.LoadingTransition_Widget_C"))
  (`UserWidget.AddToViewport` _returnvalue_5 0)
  (`UserWidget.PlayAnimation` _returnvalue_5 (`/Game/PlatformerDevelopmentKit/UI/Widgets/LoadingTransition_Widget.BlendOut` _returnvalue_5) 0.0 1 "Forward" 1.0 false)
  (`self.K2_SetActorRotation` (`self.PlayerReference`) (`KismetMathLibrary.MakeRotator` 0.0 0.0 (+ (.yaw (`KismetMathLibrary.FindLookAtRotation` (`self.K2_GetActorLocation` (`self.PlayerReference`)) (`self.K2_GetActorLocation`))) 180.0)) false)
  (`KismetSystemLibrary.Delay` 3.583)
  (`Widget.RemoveFromParent` _returnvalue_5)
  (bind _asbp_platformer_game_instance (cast `/Game/PlatformerDevelopmentKit/Base/Blueprints/BP_PlatformerGameInstance` (`GameplayStatics.GetGameInstance`)))
  (if (`/Game/PlatformerDevelopmentKit/Base/Blueprints/BP_PlatformerGameInstance.PromotSave?` _asbp_platformer_game_instance)
    (bind _returnvalue_6 (`|CreateWidget` "/Game/PlatformerDevelopmentKit/GameSaving/Widgets/SaveWindow_Widget.SaveWindow_Widget_C"))
    (`UserWidget.AddToViewport` _returnvalue_6 0)
    (`UserWidget.PlayAnimation` _returnvalue_6 (`/Game/PlatformerDevelopmentKit/GameSaving/Widgets/SaveWindow_Widget.BlendIn` _returnvalue_6) 0.0 1 "Forward" 1.0 false)
    (`WidgetBlueprintLibrary.SetInputMode_GameAndUIEx` _returnvalue null "DoNotLock" false)
    (set `PlayerController.bShowMouseCursor` true _returnvalue)
    (set `/Game/PlatformerDevelopmentKit/Base/Blueprints/BP_PlatformerGameInstance.PromotSave?` false _asbp_platformer_game_instance)))

(fn `UserConstructionScript`)