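; BP_CheckpointLantern is a checkpoint lantern that activates when the player's BP_Rabbit overlaps its capsule.
; Activation plays the lantern post animation once, shows the flame mesh and point light, and sets itself as the rabbit's current checkpoint lantern.
; A Gate, closed only after a successful rabbit cast, makes activation one-time while letting other overlapping actors pass without consuming it.
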(event `self.Capsule.OnComponentBeginOverlap`
  (params (OverlappedComponent :type "PrimitiveComponent Object Reference") (OtherActor :type "Actor Object Reference") (OtherComp :type "PrimitiveComponent Object Reference") (OtherBodyIndex :type Integer) (bFromSweep :type Boolean) (SweepResult :type "HitResult Structure (by ref)"))
  (`/Engine/EditorBlueprintResources/StandardMacros.Gate` false :!label _label
    (:`Exit`
      (bind _asbp_rabbit (cast `/Game/PlatformerDevelopmentKit/Characters/Player/Blueprints/BP_Rabbit` OtherActor))
      (set `self.PlayerReference` _asbp_rabbit)
      (`SkeletalMeshComponent.PlayAnimation` (`self.SK_Lantern`) "/Game/PlatformerDevelopmentKit/Interactables/Animations/LanternPost_Anim.LanternPost_Anim" false)
      (`SceneComponent.SetVisibility` (`self.SM_LanternFlame`) true false)
      (`SceneComponent.SetVisibility` (`self.PointLight`) true false)
      (set `/Game/PlatformerDevelopmentKit/Characters/Player/Blueprints/BP_Rabbit.CurrentCheckpointLantern` self (`self.PlayerReference`))
      (goto _label :!via `Close`))))

(fn `UserConstructionScript`)