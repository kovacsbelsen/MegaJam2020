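; BP_MainMenu is the main menu actor, which becomes the player's view target and brings up the menu interface when play begins.
; BeginPlay shows the mouse cursor in Game and UI input mode, then plays the BlendOut animation of a loading transition widget.
; After a fixed delay it removes that widget and creates the main menu widget with its MenuBlendIn animation.
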(event `self.ReceiveBeginPlay`
  (bind _returnvalue (`GameplayStatics.GetPlayerController` 0))
  (`PlayerController.SetViewTargetWithBlend` (`GameplayStatics.GetPlayerController` 0) self 0.0 "VTBlend_Linear" 0.0 false)
  (`WidgetBlueprintLibrary.SetInputMode_GameAndUIEx` _returnvalue null "DoNotLock" false)
  (set `PlayerController.bShowMouseCursor` true _returnvalue)
  (bind _returnvalue_2 (`|CreateWidget` "/Game/PlatformerDevelopmentKit/UI/Widgets/LoadingTransition_Widget.LoadingTransition_Widget_C"))
  (`UserWidget.AddToViewport` _returnvalue_2 0)
  (`UserWidget.PlayAnimation` _returnvalue_2 (`/Game/PlatformerDevelopmentKit/UI/Widgets/LoadingTransition_Widget.BlendOut` _returnvalue_2) 0.0 1 "Forward" 1.0 false)
  (`KismetSystemLibrary.Delay` 2.5)
  (`Widget.RemoveFromParent` _returnvalue_2)
  (bind _returnvalue_3 (`|CreateWidget` "/Game/PlatformerDevelopmentKit/MainMenu/Widgets/MainMenu_Widget.MainMenu_Widget_C"))
  (`UserWidget.AddToViewport` _returnvalue_3 0)
  (`UserWidget.PlayAnimation` _returnvalue_3 (`/Game/PlatformerDevelopmentKit/MainMenu/Widgets/MainMenu_Widget.MenuBlendIn` _returnvalue_3) 0.0 1 "Forward" 1.0 false))

(fn `UserConstructionScript`)