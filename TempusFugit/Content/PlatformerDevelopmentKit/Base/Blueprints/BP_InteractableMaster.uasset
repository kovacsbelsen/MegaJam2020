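; Base interactable Blueprint that registers itself and a player reference with MainChar on sphere overlap, optionally showing a button prompt.
; A Box hit fires OnInteract; if UseOnce is set, InitInteractLock then closes gates to block further use.
; End overlap still assigns itself as InteractableActor; with the prompt enabled, it hides it and fires OnInteractEnd through a DoOnce re-armed by OnInteract.
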(event `OnInteractEnd`)

(event `InitInteractLock`
  (`|ExecutionSequence`
    (:`then_0`
      (goto _label :!via `Close`))
    (:`then_1`
      (goto _label_2 :!via `Close`))
    (:`then_2`
      (goto _label_4 :!via `Close`))))

(event `self.Sphere.OnComponentBeginOverlap`
  (params (OverlappedComponent :type "PrimitiveComponent Object Reference") (OtherActor :type "Actor Object Reference") (OtherComp :type "PrimitiveComponent Object Reference") (OtherBodyIndex :type Integer) (bFromSweep :type Boolean) (SweepResult :type "HitResult Structure (by ref)"))
  (if (`self.UseOnce?`)
    (`/Engine/EditorBlueprintResources/StandardMacros.Gate` false :!label _label
      (:`Exit`
        _)))
  (bind _asmain_char (cast `/Game/JamFolder/Blueprints/MainChar` OtherActor))
  (set `self.PlayerReference` _asmain_char)
  (set `/Game/JamFolder/Blueprints/MainChar.InteractableActor` self _asmain_char)
  (if (`self.ShowButtonImage?`)
    (`SceneComponent.SetVisibility` (`self.InteractionButton`) true false)))

(event `self.Sphere.OnComponentEndOverlap`
  (params (OverlappedComponent :type "PrimitiveComponent Object Reference") (OtherActor :type "Actor Object Reference") (OtherComp :type "PrimitiveComponent Object Reference") (OtherBodyIndex :type Integer))
  (if (`self.UseOnce?`)
    (`/Engine/EditorBlueprintResources/StandardMacros.Gate` false :!label _label_2
      (:`Exit`
        _)))
  (bind _asmain_char (cast `/Game/JamFolder/Blueprints/MainChar` OtherActor))
  (set `self.PlayerReference` _asmain_char)
  (set `/Game/JamFolder/Blueprints/MainChar.InteractableActor` self _asmain_char)
  (if (`self.ShowButtonImage?`)
    (`SceneComponent.SetVisibility` (`self.InteractionButton`) false false)
    (`/Engine/EditorBlueprintResources/StandardMacros.DoOnce` true :!label _label_3
      (:`Completed`
        (`self.OnInteractEnd`)))))

(event `OnInteract`
  (goto _label_3 :!via `Reset`))

(event `self.Box.OnComponentHit`
  (params (HitComponent :type "PrimitiveComponent Object Reference") (OtherActor :type "Actor Object Reference") (OtherComp :type "PrimitiveComponent Object Reference") (NormalImpulse :type "Vector Structure") (Hit :type "HitResult Structure (by ref)"))
  (`/Engine/EditorBlueprintResources/StandardMacros.Gate` false :!label _label_4
    (:`Exit`
      (`self.OnInteract`)
      (if (`self.UseOnce?`)
        (`self.InitInteractLock`)))))

(fn `UserConstructionScript`)